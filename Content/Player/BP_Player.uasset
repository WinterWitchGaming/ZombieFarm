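; First-person player character Blueprint that handles movement, camera, shooting, reloading, damage and overlap-based interaction.
; Enhanced Input drives movement and look directly, and forwards fire and reload to the ACWeaponBase component.
; Event bindings on ACWeaponBase and ACHealthDmg update the HUD, swap the arms' animation class and rotate the arms mesh during reloads.
; Damage routes through ACHealthDmg, with death only printing a debug message, and overlapping "Interactable"-tagged actors triggers their InteractMessage.
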(event `self.ReceiveBeginPlay`
  (bind _ac_weaponbase (`self.AC_WeaponBase`))
  (bind _returnvalue (`|CreateWidget` "/Game/Player/UI/UI_HUD.UI_HUD_C"))
  (bind _output_get (set `self.HUD REF` _returnvalue))
  (`UserWidget.AddToViewport` _output_get 0)
  (add `/Game/Health_Dmg_System/ActorComponent/AC_HealthDmg.Update Health Amount` (`self.AC_HealthDmg`) (`|CreateDelegate` :!event `Update health`))
  (add `/Game/Weapons/AC_WeaponBase.onUseAmmo` _ac_weaponbase (`|CreateDelegate` :!event `Update ammo text`))
  (add `/Game/Weapons/AC_WeaponBase.On Equip gun` _ac_weaponbase (`|CreateDelegate` :!event `Equip Gun`))
  (add `/Game/Weapons/AC_WeaponBase.onStartReload` _ac_weaponbase (`|CreateDelegate` :!event `Start Reload`))
  (add `/Game/Weapons/AC_WeaponBase.onEndReload` _ac_weaponbase (`|CreateDelegate` :!event `End Reload`))
  (`/Game/Weapons/AC_WeaponBase.EquipGun` (`self.AC_WeaponBase`) "NewEnumerator2"))

(event `self.CapsuleComponent.OnComponentBeginOverlap`
  (params (OverlappedComponent :type "PrimitiveComponent Object Reference") (OtherActor :type "Actor Object Reference") (OtherComp :type "PrimitiveComponent Object Reference") (OtherBodyIndex :type Integer) (bFromSweep :type Boolean) (SweepResult :type "HitResult Structure (by ref)"))
  ;[1 1 1] Interact by running over objects
  (`/Engine/EditorBlueprintResources/StandardMacros.IsValid` OtherActor
    (:`Is Valid`
      (if (`self.ActorHasTag` OtherActor "Interactable")
        (message `/Game/Interactionsystem/BluePrintInterfaces/BPI_InteractionSystem.Interact` OtherActor)))))

(event `EnhancedInput|/Game/Player/Input/Inputactions/IA_Camera`
  (params (ActionValue :type "Vector2D Structure") (ElapsedSeconds :type "Float (double-precision)") (TriggeredSeconds :type "Float (double-precision)") (InputAction :type "InputAction Object Reference" :default "/Game/Player/Input/Inputactions/IA_Camera.IA_Camera"))
  (bind _camera_sense (`self.Camera Sense`))
  ;[1 1 1] Movement controls
  (:`Triggered`
    (`self.AddControllerYawInput` (* ActionValue_X _camera_sense))
    (`self.AddControllerPitchInput` (* ActionValue_Y _camera_sense))))

(event `EnhancedInput|/Game/Player/Input/Inputactions/IA_Move`
  (params (ActionValue :type "Vector2D Structure") (ElapsedSeconds :type "Float (double-precision)") (TriggeredSeconds :type "Float (double-precision)") (InputAction :type "InputAction Object Reference" :default "/Game/Player/Input/Inputactions/IA_Move.IA_Move"))
  ;[1 1 1] Movement controls
  (:`Triggered`
    (`self.AddMovementInput` (`self.GetActorRightVector`) ActionValue_X)
    (`self.AddMovementInput` (`self.GetActorForwardVector`) ActionValue_Y)))

(event `EnhancedInput|/Game/Player/Input/Inputactions/IA_Shoot`
  (params (ActionValue :type Boolean) (ElapsedSeconds :type "Float (double-precision)") (TriggeredSeconds :type "Float (double-precision)") (InputAction :type "InputAction Object Reference" :default "/Game/Player/Input/Inputactions/IA_Shoot.IA_Shoot"))
  (bind _ac_weaponbase (`self.AC_WeaponBase`))
  ;[1 1 1] Weapon functionality
  (:`Started`
    (`/Game/Weapons/AC_WeaponBase.Start Firing` _ac_weaponbase))
  (:`Completed`
    (`/Game/Weapons/AC_WeaponBase.Stop Firing` _ac_weaponbase)))

(event `Equip Gun`
  (params (`First Person Arms Anim BluePrint` :type "AnimInstance Class Reference"))
  ;[1 1 1] Weapon functionality
  (`SkeletalMeshComponent.SetAnimInstanceClass` (`self.First Person Mesh`) `First Person Arms Anim BluePrint`))

(event `/Game/Health_Dmg_System/BlueprintInterface/BPI_Health_Dmg_System.Damage Target`
  (params (`Damage Amount` :type "Float (double-precision)"))
  ;[1 1 1] Damage
  (bind _dead_ (`/Game/Health_Dmg_System/ActorComponent/AC_HealthDmg.Damaged Func` (`self.AC_HealthDmg`) `Damage Amount`))
  (if _dead_
    ;;[1 0 0.5497] Debug
    (`KismetSystemLibrary.PrintString` "You Are Dead")))

(event `EnhancedInput|/Game/Player/Input/Inputactions/IA_Reload`
  (params (ActionValue :type Boolean) (ElapsedSeconds :type "Float (double-precision)") (TriggeredSeconds :type "Float (double-precision)") (InputAction :type "InputAction Object Reference" :default "/Game/Player/Input/Inputactions/IA_Reload.IA_Reload"))
  ;[1 1 1] Weapon functionality
  (:`Triggered`
    (`/Game/Weapons/AC_WeaponBase.Reload` (`self.AC_WeaponBase`))))

(event `Update ammo text`
  (params (Mag :type Integer) (Reserves :type Integer))
  ;[1 1 1] Weapon functionality
  (`/Game/Player/UI/UI_HUD.Set ammo text` (`self.HUD REF`) Mag Reserves))

(event `Update health`
  (params (HealthPercentage :type "Float (double-precision)"))
  ;[1 1 1] Damage
  (`/Game/Player/UI/UI_HUD.Set Health Bar Percentage` (`self.HUD REF`) HealthPercentage))

(event `Start Reload`
  ;[1 1 1] Weapon functionality
  (`SceneComponent.K2_SetRelativeRotation` :`self` (`self.First Person Mesh`)))

(event `End Reload`
  ;[1 1 1] Weapon functionality
  (`SceneComponent.K2_SetRelativeRotation` (`self.First Person Mesh`) (struct :`Yaw` -90.0) false false))

(fn `UserConstructionScript`)