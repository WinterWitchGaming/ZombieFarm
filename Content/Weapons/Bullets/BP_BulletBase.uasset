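; Base bullet actor for weapons that damages whatever it hits and then destroys itself.
; A setter supplies damage amount and crit multiplier.
; When its sphere component hits a valid actor, it scales and rounds damage if the struck component carries a Crit tag, leaving Body hits unchanged.
; Damage goes out through an interface message, so actors not implementing it simply absorb the bullet.
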(event `/Game/Weapons/Bullets/BPI_OnBullet.Set Damage Amount`
  (params (`Damage Amount` :type "Float (double-precision)") (`Crit multiplier` :type "Float (double-precision)"))
  (set `self.Damage Amount` `Damage Amount`)
  (set `self.Crit Multiplier` `Crit multiplier`))

(event `self.Sphere.OnComponentHit`
  (params (HitComponent :type "PrimitiveComponent Object Reference") (OtherActor :type "Actor Object Reference") (OtherComp :type "PrimitiveComponent Object Reference") (NormalImpulse :type "Vector Structure") (Hit :type "HitResult Structure (by ref)"))
  (`/Engine/EditorBlueprintResources/StandardMacros.IsValid` OtherActor
    (:`Is Valid`
      (`|ExecutionSequence`
        (:`then_0`
          ;[1 1 1] Get component hit. if it is a head shot then multiply by crit modifier. if actor hit has no tag, this does nothing
          (for _array_element (`ActorComponent.ComponentTags` OtherComp)
            (switch `name` _array_element
              (:`Crit`
                (set `self.Damage Amount` (`KismetMathLibrary.Conv_IntToDouble` (`KismetMathLibrary.Round` (* (`self.Damage Amount`) (`self.Crit Multiplier`))))))
              (:`Body`
                (set `self.Damage Amount` (`self.Damage Amount`))))))
        (:`then_1`
          ;[1 1 1] Apply damage to hit actor. If actor hit does not implement this interface then nothing will happen and the bullet will be destroyed
          (message `/Game/Health_Dmg_System/BlueprintInterface/BPI_Health_Dmg_System.Damage Target` OtherActor (`self.Damage Amount`))
          (`self.Destroy Actor`))))))

(fn `Destroy Actor`
  (`self.K2_DestroyActor` self))

(fn `UserConstructionScript`)