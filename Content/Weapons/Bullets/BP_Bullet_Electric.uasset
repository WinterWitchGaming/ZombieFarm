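; BP_Bullet_Electric is an electric bullet that spreads area damage to nearby enemies when it hits an enemy.
; On a Sphere component hit against an actor tagged Enemy, it runs a multi sphere trace around the impact point, ignoring the struck actor.
; Each Enemy-tagged trace result receives fixed damage and its hit location through a DamageTarget message, with no damage applied here to the struck actor.
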(event `self.Sphere.OnComponentHit`
  (params (HitComponent :type "PrimitiveComponent Object Reference") (OtherActor :type "Actor Object Reference") (OtherComp :type "PrimitiveComponent Object Reference") (NormalImpulse :type "Vector Structure") (Hit :type "HitResult Structure (by ref)"))
  (bind (_bblockinghit _binitialoverlap _time _distance _location _impactpoint _normal _impactnormal _physmat _hitactor) (`GameplayStatics.BreakHitResult` Hit))
  (`/Engine/EditorBlueprintResources/StandardMacros.IsValid` OtherActor
    (:`Is Valid`
      (if (`self.ActorHasTag` OtherActor "Enemy")
        (bind _outhits (`KismetSystemLibrary.SphereTraceMulti` _location _location 500.0 "TraceTypeQuery4" false (`|MakeArray` _hitactor)))
        (for _array_element _outhits
          (bind (_bblockinghit_2 _binitialoverlap_2 _time_2 _distance_2 _location_2 _impactpoint_2 _normal_2 _impactnormal_2 _physmat_2 _hitactor_2) (`GameplayStatics.BreakHitResult` _array_element))
          (`/Engine/EditorBlueprintResources/StandardMacros.IsValid` _hitactor_2
            (:`Is Valid`
              (if (`self.ActorHasTag` _hitactor_2 "Enemy")
                (message `/Game/Health_Dmg_System/BlueprintInterface/BPI_Health_Dmg_System.Damage Target` _hitactor_2 20.0 _location_2)))))))))

(fn `UserConstructionScript`
  (`parent.UserConstructionScript`))