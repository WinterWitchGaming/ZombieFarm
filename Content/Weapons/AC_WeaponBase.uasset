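; Skeletal mesh weapon component that handles equipping, firing, recoil and reloading, configured per gun from DT_Guns.
; StartFiring routes to semi, three-round burst or timer-looped full-auto modes, each gated by DoOnce.
; Each shot spawns a projectile at the muzzle aimed along a camera trace, passes it damage values, and plays montage-driven recoil with camera shake.
; Delayed reloads pool magazine and reserve ammo, with dispatchers broadcasting ammo, equip and reload changes.
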(event `Stop Firing`
  (`KismetSystemLibrary.K2_ClearAndInvalidateTimerHandle` (`self.Full Auto Timer`)))

(event `Start Firing`
  (bind (_fireselect _damageamount _critmultiplier _firerate _burstdelay) (break `/Game/Weapons/Strut_Enum/S_WeaponVariables` (`self.Gun Variables`)))
  (if (> (`self.Mag`) 0)
    (switch `/Game/Weapons/Strut_Enum/E_FireSelect` _fireselect
      (:`NewEnumerator0`
        (`/Engine/EditorBlueprintResources/StandardMacros.DoOnce` false :!label _label
          (:`Completed`
            (bind _returnvalue (`KismetSystemLibrary.K2_SetTimer` null "Spawn bullet" _firerate true (* _firerate -1.0)))
            (set `self.Full Auto Timer` _returnvalue)
            (`KismetSystemLibrary.Delay` _firerate)
            (goto _label :!via `Reset`))))
      (:`NewEnumerator1`
        (`/Engine/EditorBlueprintResources/StandardMacros.DoOnce` false :!label _label_2
          (:`Completed`
            (`self.Spawn bullet`)
            (`KismetSystemLibrary.Delay` _burstdelay)
            (`self.Spawn bullet`)
            (`KismetSystemLibrary.Delay` _burstdelay)
            (`self.Spawn bullet`)
            (`KismetSystemLibrary.Delay` _burstdelay)
            (`KismetSystemLibrary.Delay` _firerate)
            (goto _label_2 :!via `Reset`))))
      (:`NewEnumerator2`
        (`/Engine/EditorBlueprintResources/StandardMacros.DoOnce` false :!label _label_3
          (:`Completed`
            (`self.Spawn bullet`)
            (`KismetSystemLibrary.Delay` _firerate)
            (goto _label_3 :!via `Reset`)))))
    (else
      (`self.Reload`))))

(event `Play Fire Mont`
  (`|PlayMontage` self "/Game/Weapons/Revolver/Animations/Revolver_Fire_Montage.Revolver_Fire_Montage"
    (:`then`
      (`self.Recoil`))))

(event `Reload`
  (if (and (< (`self.Mag`) (`self.Max Mag Size`)) (> (`self.Reserves`) 0) (not (`self.Reloading?`)))
    (`self.onStartReload`)
    (`self.Start reload`)
    (`KismetSystemLibrary.Delay` (`.ReloadDelay_25_E412C5C648AB176E0B241D95D20D2664` (break `/Game/Weapons/Strut_Enum/S_WeaponVariables` (`self.Gun Variables`))))
    (`self.onEndReload`)
    (`KismetSystemLibrary.Delay` 0.7)
    (`self.EndReload`)))

(fn `EndReload`
  (set `self.Reloading?` false)
  (if (< (`self.Reserves`) (`self.Max Mag Size`))
    (set `self.Mag` (`self.Reserves`))
    (set `self.Reserves` 0)
    (else
      (set `self.Reserves` (- (`self.Reserves`) (`self.Max Mag Size`)))
      (set `self.Mag` (`self.Max Mag Size`))))
  (`self.onUseAmmo` (`self.Mag`) (`self.Reserves`)))

(fn `EquipGun`
  (params (GunName :type "/Game/Weapons/E_GunNames Enum" :default "NewEnumerator0"))
  (bind (_fireselect _damageamount _critmultiplier _firerate _burstdelay _bullettype _magsize _reserves) (break `/Game/Weapons/Strut_Enum/S_WeaponVariables` (`self.Gun Variables`)))
  (bind _returnvalue (`|GetDataTableRow` "/Game/Weapons/DT_Guns.DT_Guns" (`KismetStringLibrary.Conv_StringToName` (`|GetEnumeratorNameAsString` GunName)))
    (:`then`
      (bind _output_get (set `self.Gun Variables` _returnvalue))
      (`self.SetSkeletalMeshAsset` self (`.GunMesh_39_1BD36EF64335F88854FD5CA1D6F4DE36` (break `/Game/Weapons/Strut_Enum/S_WeaponVariables` _output_get)))
      (`self.On Equip gun`)
      (bind _output_get_2 (set `self.Mag` _magsize))
      (set `self.Max Mag Size` _output_get_2)
      (set `self.Reserves` _reserves)
      (`self.onUseAmmo` (`self.Mag`) (`self.Reserves`)))))

(fn `Recoil`
  (bind _returnvalue (`GameplayStatics.GetPlayerController` 0))
  (bind (_fireselect _damageamount _critmultiplier _firerate _burstdelay _bullettype _magsize _reserves _reloaddelay _recoilyawmin _recoilyawmax _recoilpitchmin _recoilpitchmax) (break `/Game/Weapons/Strut_Enum/S_WeaponVariables` (`self.Gun Variables`)))
  (`LegacyCameraShake.StartLegacyCameraShake` (`GameplayStatics.GetPlayerCameraManager` 0) "/Game/Weapons/CameraShake/CS_WeaponFire.CS_WeaponFire_C")
  (`PlayerController.AddPitchInput` _returnvalue (* (`KismetMathLibrary.RandomFloatInRange` _recoilpitchmin _recoilpitchmax) -1.0))
  (`PlayerController.AddYawInput` _returnvalue (* (`KismetMathLibrary.RandomFloatInRange` _recoilyawmin _recoilyawmax) -1.0)))

(fn `Spawn bullet`
  (bind _returnvalue (`GameplayStatics.GetPlayerCameraManager` 0))
  (bind _mag (`self.Mag`))
  (bind (_fireselect _damageamount _critmultiplier _firerate _burstdelay _bullettype) (break `/Game/Weapons/Strut_Enum/S_WeaponVariables` (`self.Gun Variables`)))
  (bind _returnvalue_2 (`self.GetSocketLocation` self "Muzzle"))
  (bind _returnvalue_3 (`Actor.K2_GetActorLocation` _returnvalue))
  (bind _returnvalue_4 (`self.GetSocketLocation` self "Muzzle"))
  (bind _returnvalue_5 (+ _returnvalue_3 (* (`Actor.GetActorForwardVector` _returnvalue) 1000.0)))
  ;[1 1 1] Get a line trace out from the player to direct the bullet. If it does not hit anything then direct the bullet toward it's max range
  (if (and (> _mag 0) (not (`self.Reloading?`)))
    (bind _result (`/Engine/EditorBlueprintResources/StandardMacros.DecrementInt` _mag)
      (:`  `
        (`self.onUseAmmo` _result (`self.Reserves`))
        (`self.Play Fire Mont`)
        (bind (_outhit _returnvalue_6) (`KismetSystemLibrary.LineTraceSingle` _returnvalue_3 _returnvalue_5 "TraceTypeQuery1"))
        (if _returnvalue_6
          (bind _returnvalue_7 (`|SpawnActorFromClass` _bullettype (`KismetMathLibrary.MakeTransform` _returnvalue_2 (`KismetMathLibrary.FindLookAtRotation` _returnvalue_2 (`.Location` (`GameplayStatics.BreakHitResult` _outhit)))) "Undefined" "MultiplyWithRoot" null null))
          (`/Engine/EditorBlueprintResources/StandardMacros.IsValid` _returnvalue_7
            (:`Is Valid`
              (message `/Game/Weapons/Bullets/BPI_OnBullet.Set Damage Amount` _returnvalue_7 _damageamount _critmultiplier)))
          (else
            (bind _returnvalue_8 (`|SpawnActorFromClass` _bullettype (`KismetMathLibrary.MakeTransform` _returnvalue_4 (`KismetMathLibrary.FindLookAtRotation` _returnvalue_4 _returnvalue_5)) "Undefined" "MultiplyWithRoot" null null))
            (`/Engine/EditorBlueprintResources/StandardMacros.IsValid` _returnvalue_8
              (:`Is Valid`
                (message `/Game/Weapons/Bullets/BPI_OnBullet.Set Damage Amount` _returnvalue_8 _damageamount _critmultiplier)))))))
    (else
      (`self.Reload`))))

(fn `Start reload`
  (bind _output_get (set `self.Reserves` (+ (`self.Mag`) (`self.Reserves`))))
  (bind _output_get_2 (set `self.Mag` 0))
  (`self.onUseAmmo` _output_get_2 _output_get)
  (set `self.Reloading?` true))