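; Game mode for the hedge maze that runs score-gated rooms of enemy spawning and updates the score UI.
; A looping timer spawns enemies at random from accumulated player-proximate spawners, capped by enemy count.
; Kills build a timed score multiplier and toughen later spawns.
; A kill after reaching the target wipes enemies, opens the numbered door and, behind a DoOnce reset by StartNextRoom, raises the target and spawn rate.
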(event `OpenDoors`
  (bind _outactors (`GameplayStatics.GetAllActorsOfClass` "/Game/Maps/MapFunctionality/BP_Door.BP_Door_C"))
  (for _array_element _outactors
    (if (== (`/Game/Maps/MapFunctionality/BP_Door.Door Number` _array_element) (`self.Door to open`))
      (`/Game/Maps/MapFunctionality/BP_Door.Open Door` _array_element))))

(event `self.ReceiveBeginPlay`
  ;[1 1 1] Begin play
  (bind _returnvalue (`|CreateWidget` "/Game/Player/UI/UI_GameModeUI.UI_GameModeUI_C"))
  (bind _output_get (set `self.UI REF` _returnvalue))
  (`UserWidget.AddToViewport` _output_get 0)
  (bind _outactors (`GameplayStatics.GetAllActorsOfClass` "/Game/Enemies/Spawner/BP_EnemySpawner.BP_EnemySpawner_C"))
  (set `self.Enemy Spawners` _outactors)
  (`self.Start Spawning Enemies`)
  (bind _outactors_2 (`GameplayStatics.GetAllActorsOfClass` "/Game/Enemies/BP_Enemy_Base.BP_Enemy_Base_C"))
  (set `self.Enemies in map` (`KismetArrayLibrary.Array_Length` _outactors_2)))

(event `/Game/FrameWork/GameModes/BPI_OnGameMode.Enemy Killed`
  ;[1 1 1] Enemy Killed
  (bind _result (`/Engine/EditorBlueprintResources/StandardMacros.DecrementInt` (`self.Enemies in map`))
    (:`  `
      (if (< (`self.Score`) (`self.Max Score Needed`))
        (`|ExecutionSequence`
          (:`then_0`
            (set `self.Score Multiplier` (`KismetMathLibrary.FClamp` (+ (`self.Score Multiplier`) 0.1) 1.0 5.0))
            (`self.Update Score`)
            (bind _output_get (set `self.Score multiplier reset cool down` 5))
            (`/Game/Player/UI/UI_GameModeUI.Update cool down timer` (`self.UI REF`) (`KismetMathLibrary.Conv_IntToDouble` _output_get))
            (bind _returnvalue (`KismetSystemLibrary.K2_SetTimerDelegate` (delegate `Reduce score multiplier cooldown`) 1.0 true 1.5))
            (set `self.Score reset timer` _returnvalue))
          (:`then_1`
            (if (and (< _result 100) (not (`KismetSystemLibrary.K2_IsTimerActiveHandle` (`self.Enemy Spawner timer`))))
              (`self.Start Spawning Enemies`)))
          (:`then_2`
            (set `self.input health` (`KismetMathLibrary.FClamp` (+ (`self.input health`) 10.0) 0.0 150.0))
            (set `self.Input Walk speed` (+ (`self.Input Walk speed`) 10.0))))
        (else
          (`KismetSystemLibrary.K2_ClearAndInvalidateTimerHandle` (`self.Enemy Spawner timer`))
          (`|ExecutionSequence`
            (:`then_0`
              (bind _outactors (`GameplayStatics.GetAllActorsOfClass` "/Game/Enemies/BP_Enemy_Base.BP_Enemy_Base_C"))
              (for _array_element _outactors
                (`/Engine/EditorBlueprintResources/StandardMacros.IsValid` _array_element
                  (:`Is Valid`
                    (message `/Game/Health_Dmg_System/BlueprintInterface/BPI_Health_Dmg_System.Damage Target` _array_element 9999.0)))))
            (:`then_1`
              (bind _outactors_2 (`GameplayStatics.GetAllActorsOfClass` "/Game/Maps/MapFunctionality/BP_Door.BP_Door_C"))
              (for _array_element_2 _outactors_2
                (if (== (`/Game/Maps/MapFunctionality/BP_Door.Door Number` _array_element_2) (`self.Door to open`))
                  (`/Game/Maps/MapFunctionality/BP_Door.Open Door` _array_element_2))))
            (:`then_2`
              (`/Engine/EditorBlueprintResources/StandardMacros.DoOnce` false :!label _label
                (:`Completed`
                  (`/Engine/EditorBlueprintResources/StandardMacros.IncrementInt` (`self.Door to open`)
                    (:`  `
                      (set `self.Score` 0.0)
                      (set `self.Max Score Needed` (+ (`self.Max Score Needed`) 10.0))
                      (`/Game/Player/UI/UI_GameModeUI.UpdateScore` (`self.UI REF`) (`self.Score`) (`self.Max Score Needed`) (`self.Score Multiplier`))
                      (set `self.Enemy Spawn Speed` (`KismetMathLibrary.FClamp` (- (`self.Enemy Spawn Speed`) 0.5) 1.0 2.0)))))))))))))

(event `Reduce score multiplier cooldown`
  ;[1 1 1] Enemy Killed
  (bind _result (`/Engine/EditorBlueprintResources/StandardMacros.DecrementInt` (`self.Score multiplier reset cool down`))
    (:`  `
      (`/Game/Player/UI/UI_GameModeUI.Update cool down timer` (`self.UI REF`) (`KismetMathLibrary.Conv_IntToDouble` _result))
      (if (<= _result 0)
        (`KismetSystemLibrary.K2_ClearAndInvalidateTimerHandle` (`self.Score reset timer`))
        (bind _output_get (set `self.Score Multiplier` 1.0))
        (`/Game/Player/UI/UI_GameModeUI.UpdateScore` (`self.UI REF`) (`self.Score`) (`self.Max Score Needed`) _output_get)))))

(event `Reset start next room`
  ;[1 1 1] Enemy Killed
  (goto _label :!via `Reset`))

(event `Spawn enemy`
  (bind _nearby_spawners (`self.Nearby spawners`))
  (bind _outitem (`KismetArrayLibrary.Array_Random` _nearby_spawners))
  ;[1 1 1] Spawn enemy
  (if (not (`self.game over?`))
    (if (< (`self.Enemies in map`) 100)
      (for _array_element (`self.Enemy Spawners`)
        (if (<= (`self.GetDistanceTo` _array_element (`GameplayStatics.GetPlayerCharacter` 0)) 3000.0)
          (`KismetArrayLibrary.Array_Add` (`self.Nearby spawners`) _array_element)))
      (if (> (`KismetArrayLibrary.Array_Length` _nearby_spawners) 0)
        (`/Engine/EditorBlueprintResources/StandardMacros.IsValid` _outitem
          (:`Is Valid`
            (`/Game/Enemies/Spawner/BP_EnemySpawner.Spawn enemy` _outitem (`self.input health`) (`self.Input Walk speed`))
            (`/Engine/EditorBlueprintResources/StandardMacros.IncrementInt` (`self.Enemies in map`)))))
      (else
        (`KismetSystemLibrary.K2_ClearAndInvalidateTimerHandle` (`self.Enemy Spawner timer`))))
    (else
      (`KismetSystemLibrary.K2_ClearAndInvalidateTimerHandle` (`self.Enemy Spawner timer`)))))

(event `Start Spawning Enemies`
  ;[1 1 1] Spawn enemy
  (if (not (`self.game over?`))
    (bind _outactors (`GameplayStatics.GetAllActorsOfClass` "/Game/Enemies/Spawner/BP_EnemySpawner.BP_EnemySpawner_C"))
    (set `self.Enemy Spawners` _outactors)
    (bind _returnvalue (`KismetSystemLibrary.K2_SetTimerDelegate` (delegate `Spawn enemy`) (`self.Enemy Spawn Speed`) true))
    (set `self.Enemy Spawner timer` _returnvalue)))

(event `/Game/FrameWork/GameModes/BPI_OnGameMode.Player died`
  ;[1 1 1] Spawn enemy
  (`KismetSystemLibrary.K2_ClearAndInvalidateTimerHandle` (`self.Enemy Spawner timer`))
  (`Widget.RemoveFromParent` (`self.UI REF`)))

(event `/Game/FrameWork/GameModes/BPI_OnGameMode.Start Next room`
  ;[1 1 1] Spawn enemy
  (`KismetSystemLibrary.Delay` 1.0)
  (`self.Start Spawning Enemies`)
  (`self.Reset start next room`))

(fn `Update Score`
  (bind _output_get (set `self.Score` (+ (`self.Score`) (* (`self.Score Multiplier`) 5.0))))
  (`/Game/Player/UI/UI_GameModeUI.UpdateScore` (`self.UI REF`) _output_get (`self.Max Score Needed`) (`self.Score Multiplier`)))

(fn `UserConstructionScript`)