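; BP_MenuPawn is a main menu pawn that moves between indexed camera positions while facing a focal point.
; BeginPlay caches the first BP_MEnuCameraFocalPoint, which Tick keeps the pawn rotated toward, then calls MoveCamera.
; A and D step the clamped camera index and call MoveCamera again.
; MoveCamera finds the BP_CameraPath with that index and runs a timeline that lerps from the current location toward it.
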(event `self.ReceiveTick`
  (params (DeltaSeconds :type "Float (single-precision)"))
  (bind _focalpoint (`self.FocalPoint`))
  (`/Engine/EditorBlueprintResources/StandardMacros.IsValid` _focalpoint
    (:`Is Valid`
      (`self.K2_SetActorRotation` (`KismetMathLibrary.FindLookAtRotation` (`self.K2_GetActorLocation`) (`self.K2_GetActorLocation` _focalpoint))))))

(event `self.ReceiveBeginPlay`
  (`|ExecutionSequence`
    (:`then_0`
      (bind _outactors (`GameplayStatics.GetAllActorsOfClass` "/Game/FrameWork/MainMenu/BP_MEnuCameraFocalPoint.BP_MEnuCameraFocalPoint_C"))
      (set `self.FocalPoint` (`|GetArrayItem` _outactors)))
    (:`then_1`
      (`self.Move Camera`))))

(event `Move Camera`
  (`KismetArrayLibrary.Array_Clear` (`self.Camera to move to`))
  (bind _outactors (`GameplayStatics.GetAllActorsOfClass` "/Game/FrameWork/MainMenu/BP_CameraPath.BP_CameraPath_C"))
  (for _array_element _outactors
    (if (== (`/Game/FrameWork/MainMenu/BP_CameraPath.CameraPath Index` _array_element) (`self.Camera LOC Index`))
      (`KismetArrayLibrary.Array_Add` (`self.Camera to move to`) _array_element)
      (bind (_direction _newtrack_0) (`Timeline|Timeline` :!via `PlayFromStart`)
        (:`Update`
          (`self.K2_SetActorLocation` (`KismetMathLibrary.VLerp` (`self.K2_GetActorLocation`) (`self.K2_GetActorLocation` (`|GetArrayItem` (`self.Camera to move to`))) _newtrack_0)))))))

(event `Key|A`
  (params (Key :type "Key Structure"))
  (bind _returnvalue (- (`self.Camera LOC Index`) 1))
  (:`Pressed`
    (set `self.Camera LOC Index` (`KismetMathLibrary.Clamp` _returnvalue -2 _returnvalue))
    (`self.Move Camera`)))

(event `Key|D`
  (params (Key :type "Key Structure"))
  (:`Pressed`
    (set `self.Camera LOC Index` (`KismetMathLibrary.Clamp` (+ (`self.Camera LOC Index`) 1) -1 2))
    (`self.Move Camera`)))

(fn `UserConstructionScript`)