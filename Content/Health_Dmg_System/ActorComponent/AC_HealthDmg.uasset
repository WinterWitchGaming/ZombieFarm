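; Actor component that tracks health, applies damage and optionally regenerates health after a delay.
; DamagedFunc subtracts damage, reports whether health is depleted and extends a capped regen delay with each hit.
; A one-second looping timer counts that delay down, then a second timer restores health until it reaches the maximum.
; Health changes broadcast a normalized value through UpdateHealthAmount, with toggleable debug prints.
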(event `Start health regen count down`
  (if (`self.Should Regen Health?`)
    (`KismetSystemLibrary.K2_ClearAndInvalidateTimerHandle` (`self.Health Regen Count down timer`))
    (`KismetSystemLibrary.K2_ClearAndInvalidateTimerHandle` (`self.Regen health timer`))
    (bind _returnvalue (`KismetSystemLibrary.K2_SetTimerDelegate` (delegate `Health regen count down`) 1.0 true -1.0))
    (set `self.Health Regen Count down timer` _returnvalue)))

(event `Health regen count down`
  (bind _regen_speed (`self.Regen Speed`))
  (bind _result (`/Engine/EditorBlueprintResources/StandardMacros.DecrementInt` (`self.Time before health regens (Seconds)`))
    (:`  `
      (`self.Debug health regen timer`)
      (if (<= _result 0)
        (`KismetSystemLibrary.K2_ClearAndInvalidateTimerHandle` (`self.Health Regen Count down timer`))
        (bind _returnvalue (`KismetSystemLibrary.K2_SetTimer` null "Regen Health" _regen_speed true (* _regen_speed -1.0)))
        (set `self.Regen health timer` _returnvalue)))))

(fn `Damaged Func`
  (params (`Dmg Amount` :type "Float (double-precision)"))
  (returns (`Dead?` :type Boolean))
  (if (> (`self.Health`) 0.0)
    (bind _output_get (set `self.Health` (- (`self.Health`) `Dmg Amount`)))
    (`self.Get health percentage`)
    (`self.Debug health amount`)
    (`self.Debug Dmg Amount` `Dmg Amount`)
    (set `self.Time before health regens (Seconds)` (`KismetMathLibrary.Clamp` (+ (`self.Time before health regens (Seconds)`) (`self.Time to add per hit (Seconds)`)) 0 (`self.Max time before regen`)))
    (`self.Start health regen count down`)
    (return (<= _output_get 0.0))))

(fn `Debug Dmg Amount`
  (params (`Dmg amount` :type "Float (double-precision)"))
  (if (`self.Debug Dmg Amount?`)
    (`KismetSystemLibrary.PrintString` (`KismetStringLibrary.Concat_StrStr` "Damage Amount: " (`KismetStringLibrary.Conv_DoubleToString` `Dmg amount`)))))

(fn `Debug health amount`
  (if (`self.Debug health amount?`)
    (`KismetSystemLibrary.PrintString` (`KismetStringLibrary.Concat_StrStr` "Health Amount: " (`KismetStringLibrary.Conv_DoubleToString` (`self.Health`))))))

(fn `Debug health regen timer`
  (if (`self.Debug health regen timer?`)
    (`KismetSystemLibrary.PrintString` (`KismetStringLibrary.Concat_StrStr` "Health Regen Timer: " (`KismetStringLibrary.Conv_IntToString` (`self.Time before health regens (Seconds)`))))))

(fn `Get health percentage`
  (`self.Update Health Amount` self (/ (`self.Health`) (`self.Max Health`))))

(fn `Regen Health`
  (bind _output_get (set `self.Health` (+ (`self.Health`) (`self.Regen Amount`))))
  (`self.Get health percentage`)
  (if (>= _output_get (`self.Max Health`))
    (`KismetSystemLibrary.K2_ClearAndInvalidateTimerHandle` (`self.Regen health timer`))))