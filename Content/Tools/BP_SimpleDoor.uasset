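; BP_SimpleDoor is a door actor that swings open automatically when the player enters its Box trigger.
; On overlap by BP_Player, it plays an attenuated creak sound and runs a Timeline that lerps both static meshes' relative yaw from closed to a quarter turn.
; End overlap reverses the Timeline to close the door, without the player check or a sound call.
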(event `self.Box.OnComponentBeginOverlap`
  (params (OverlappedComponent :type "PrimitiveComponent Object Reference") (OtherActor :type "Actor Object Reference") (OtherComp :type "PrimitiveComponent Object Reference") (OtherBodyIndex :type Integer) (bFromSweep :type Boolean) (SweepResult :type "HitResult Structure (by ref)"))
  (cast `/Game/Player/BP_Player` OtherActor)
  (`GameplayStatics.PlaySoundAtLocation` "/Game/Sound/door-creaking-121673_Cue.door-creaking-121673_Cue" (`SceneComponent.K2_GetComponentLocation` (`self.DefaultSceneRoot`)) (struct) 1.0 1.0 0.0 "/Game/FrameWork/Audio/Attenuation/AT_ZombieMoises.AT_ZombieMoises" null null null)
  (bind (_direction _alpha) (`Timeline|Timeline` :!label _label)
    (:`Update`
      (bind _returnvalue (`KismetMathLibrary.Lerp` 0.0 90.0 _alpha))
      (`SceneComponent.K2_SetRelativeRotation` (`self.StaticMesh1`) (`KismetMathLibrary.MakeRotator` 0.0 0.0 _returnvalue) false false)
      (`SceneComponent.K2_SetRelativeRotation` (`self.StaticMesh`) (`KismetMathLibrary.MakeRotator` 0.0 0.0 _returnvalue) false false))))

(event `self.Box.OnComponentEndOverlap`
  (params (OverlappedComponent :type "PrimitiveComponent Object Reference") (OtherActor :type "Actor Object Reference") (OtherComp :type "PrimitiveComponent Object Reference") (OtherBodyIndex :type Integer))
  (goto _label :!via `Reverse`))

(fn `UserConstructionScript`)