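; Procedural modular wall tool that tiles an instanced mesh along local Y to fill the distance set by LastInstanceEnd.
; Construction script optionally regenerates it: clear, measure module length from bounds, then place modules and periodic connector meshes with per-mesh transforms.
; Each module gets random decorations as static mesh components, drawn from a seeded stream for repeatable layouts; RandomPosition rerolls the seed.
; The anti-decoration volume check is defined but never called.
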(fn `AddDecorationMesh`
  (params (A :type "Vector Structure") (RandomlyPickMesh :type "StaticMesh Object Reference") (RandomlyPickedTransform :type "Transform Structure (by ref)"))
  (bind _returnvalue (`AddComponent|NODE_AddStaticMeshComponent-0`))
  (`KismetArrayLibrary.Array_AddUnique` (`self.SpawnedDecoration`) _returnvalue)
  (`StaticMeshComponent.SetStaticMesh` _returnvalue RandomlyPickMesh)
  (`SceneComponent.SetWorldScale3D` _returnvalue (1.0 1.0 1.0))
  (`SceneComponent.K2_AddLocalTransform` _returnvalue RandomlyPickedTransform false true)
  (`SceneComponent.K2_AddLocalTransform` _returnvalue (`KismetMathLibrary.MakeTransform` (+ (* A (1.0 -1.0 1.0)) (`KismetMathLibrary.MakeVector` 0.0 (`self.MeshLength`))) (struct :`Yaw` 180.0)) false true))

(fn `AddDecorations`
  (params (ModuleTransform :type "Transform Structure") (MeshLength :type "Float (double-precision)") (Index :type Integer))
  (locals (RandomlyPickMesh :type "StaticMesh Object Reference") (RandomlyPickedTansform :type "Transform Structure") (DecorationLocationWorld :type "Vector Structure" :default (0.0 0.0 0.0)))
  (`|ExecutionSequence`
    (:`then_0`
      (set `self.WallExtentsX` (.x (`.BoxExtent` (`KismetMathLibrary.BreakBoxSphereBounds` (`StaticMesh.GetBounds` (`self.MeshModule`)))))))
    (:`then_1`
      (bind _output_get (set `self.DeacorationCount` (`KismetMathLibrary.RandomIntegerInRangeFromStream` (`self.RandomStream`) (`self.MinDecoration`) (`self.MaxDecoration`))))
      (for _ (range _output_get)
        (`|ExecutionSequence`
          (:`then_0`
            ;[1 1 1] Pick a random decoration mesh
            (set `self.RandomlyPickedIndex` (`KismetMathLibrary.RandomIntegerInRangeFromStream` (`self.RandomStream`) 0 (- (`KismetArrayLibrary.Array_Length` (`self.DecorationMeshes`)) 1))))
          (:`then_1`
            (set `local.RandomlyPickMesh` (`|GetArrayItem` (`self.DecorationMeshes`) (`self.RandomlyPickedIndex`))))
          (:`then_2`
            ;[1 1 1] Find a matching trasform - or just use identity (nutral)
            (if (< (`self.RandomlyPickedIndex`) (`KismetArrayLibrary.Array_Length` (`self.DecorartionTransform`)))
              (set `local.RandomlyPickedTansform` (`|GetArrayItem` (`self.DecorartionTransform`) (`self.RandomlyPickedIndex`)))
              (else
                (set `local.RandomlyPickedTansform` (`KismetMathLibrary.MakeTransform` (0.0 0.0 0.0))))))
          (:`then_3`
            (bind _localposition (`self.Get Random Point Within Module` ModuleTransform (`|GetArrayItem` (`self.MeshConnector`))))
            (set `local.DecorationLocationWorld` (`KismetMathLibrary.TransformLocation` (`self.GetTransform`) _localposition))
            (`self.AddDecorationMesh` _localposition (`local.RandomlyPickMesh`) (`local.RandomlyPickedTansform`))))))))

(fn `AddModule`
  (params (`Instance Index` :type Integer) (MeshLength :type "Float (double-precision)") (FillOffset :type Boolean))
  (returns (Index :type Integer) (Transform :type "Transform Structure"))
  (bind _returnvalue (`KismetMathLibrary.MakeTransform` (`KismetMathLibrary.MakeVector` 0.0 (* (* `Instance Index` MeshLength) -1.0)) (struct) (1.0 1.0 1.0)))
  (if (not FillOffset)
    (`InstancedStaticMeshComponent.AddInstance` (`self.InstanceGroupWall`) _returnvalue false))
  (if (and (== (mod (+ `Instance Index` (`self.ConnectorIndexStart`)) (+ (`self.ConnectorIndexOffset`) 1)) 0) (>= `Instance Index` (`self.ConnectorIndexStart`)))
    (for (_array_element _array_index) (`self.MeshConnectorInstance`)
      (bind (_output_location _output_rotation _output_scale) (`KismetMathLibrary.BreakTransform` (`|GetArrayItem` (`self.ConnectorTransform`) _array_index)))
      (`InstancedStaticMeshComponent.AddInstance` _array_element (`KismetMathLibrary.MakeTransform` (+ (.location _returnvalue) _output_location) (struct) _output_scale) false)))
  (return 0 _returnvalue))

(fn `CalcDistanceToEnd`
  (returns (ReturnValue :type "Float (double-precision)"))
  (bind (_lastinstanceend_x _lastinstanceend_y) (`KismetMathLibrary.BreakVector` (`self.LastInstanceEnd`)))
  (return (`KismetMathLibrary.FMax` _lastinstanceend_y 1.0)))

(fn `CalcInstanceCount`
  (params (DistanceToEnd :type "Float (double-precision)") (MeshLength :type "Float (double-precision)"))
  (returns (InstanceCount :type Integer))
  (return (`KismetMathLibrary.FFloor` (/ DistanceToEnd MeshLength))))

(fn `CalcMeshLength`
  (returns (ReturnValue :type "Float (double-precision)"))
  (bind (_returnvalue_origin _returnvalue_boxextent) (`KismetMathLibrary.BreakBoxSphereBounds` (`StaticMesh.GetBounds` (`self.MeshModule`))))
  (return (+ (* (.y _returnvalue_boxextent) 2.0) (`self.MainMeshOffset`))))

(fn `Clear`
  (`|ExecutionSequence`
    (:`then_0`
      (`KismetMathLibrary.SetRandomStreamSeed` (`self.RandomStream`) (`self.Seed`)))
    (:`then_1`
      (`ActorComponent.K2_DestroyComponent` (`self.SpawnedDecoration`))
      (`KismetArrayLibrary.Array_Clear` (`self.SpawnedDecoration`)))
    (:`then_2`
      (`InstancedStaticMeshComponent.ClearInstances` (`self.InstanceGroupWall`)))
    (:`then_3`
      (for _array_element (`self.MeshConnectorInstance`)
        (`InstancedStaticMeshComponent.ClearInstances` _array_element))
      (`KismetArrayLibrary.Array_Clear` (`self.MeshConnectorInstance`)))))

(fn `Get Random DecorationMesh`
  (returns (Output :type "StaticMesh Object Reference"))
  (bind _decorationmeshes (`self.DecorationMeshes`))
  (return (`|GetArrayItem` _decorationmeshes (- (`KismetMathLibrary.RandomIntegerInRangeFromStream` (`self.RandomStream`) 1 (`KismetArrayLibrary.Array_Length` _decorationmeshes)) 1))))

(fn `Get Random Point Within Module`
  (params (T :type "Transform Structure (by ref)") (Target :type "StaticMesh Object Reference"))
  (returns (LocalPosition :type "Vector Structure"))
  (locals (RandomX :type "Float (single-precision)" :default 0.0) (RandomZ :type "Float (single-precision)" :default 0.0))
  (bind (_returnvalue_origin _returnvalue_boxextent) (`KismetMathLibrary.BreakBoxSphereBounds` (`StaticMesh.GetBounds` (`self.MeshModule`))))
  (`|ExecutionSequence`
    (:`then_0`
      (set `local.RandomX` (`KismetMathLibrary.RandomFloatInRangeFromStream` (`self.RandomStream`) -0.7 0.7)))
    (:`then_1`
      (set `local.RandomZ` (`KismetMathLibrary.RandomFloatInRangeFromStream` (`self.RandomStream`) -0.1 0.7)))
    (:`then_2`
      (return (`KismetMathLibrary.TransformLocation` T (* (+ (* (`KismetMathLibrary.MakeVector` 0.0 (`local.RandomX`) (`local.RandomZ`)) _returnvalue_boxextent) _returnvalue_boxextent) (.scale T)))))))

(fn `Initialize`
  (`|ExecutionSequence`
    (:`then_0`
      (`StaticMeshComponent.SetStaticMesh` (`self.InstanceGroupWall`) (`self.MeshModule`))
      (for _array_element (`self.MeshConnector`)
        (bind _returnvalue (`AddComponent|NODE_AddInstancedStaticMeshComponent-0` :`RelativeTransform` (`KismetMathLibrary.MakeTransform` (0.0 0.0 0.0) (struct :`Yaw` 180.0))))
        (`StaticMeshComponent.SetStaticMesh` _returnvalue _array_element)
        (`KismetArrayLibrary.Array_AddUnique` (`self.MeshConnectorInstance`) _returnvalue)))
    (:`then_1`
      (set `self.MeshLength` (`self.CalcMeshLength`)))
    (:`then_2`
      (set `self.DistanceToEnd` (`self.CalcDistanceToEnd`)))))

(fn `IsPointWithinAntiDecorationVolumes`
  (params (PointWorld :type "Vector Structure"))
  (returns (IsWithin :type Boolean))
  (bind _returnvalue (`KismetMathLibrary.MakeVector` (.x PointWorld) (* (.y PointWorld) -1.0) (.z PointWorld)))
  (for _array_element _
    (`KismetSystemLibrary.PrintString` (`KismetStringLibrary.Conv_VectorToString` _returnvalue))
    (bind _brushcomponent (`Brush.BrushComponent` _array_element))
    (bind _returnvalue_2 (`SceneComponent.K2_GetComponentToWorld` _brushcomponent))
    (`KismetSystemLibrary.PrintString` (`KismetStringLibrary.Conv_TransformToString` _returnvalue_2))
    (if (`KismetMathLibrary.IsPointInBoxWithTransform` _returnvalue _returnvalue_2 (`.BoxExtent` (`KismetSystemLibrary.GetComponentBounds` _brushcomponent)))
      (return true)))
  (return false))

(fn `RandomPosition`
  (set `self.Seed` (`KismetMathLibrary.RandomInteger` 4354657))
  (`self.RunWallGeneration`))

(fn `RunWallGeneration`
  (locals (NumDecorationsToClear :type Integer :default 0))
  (bind _returnvalue (- (`self.InstanceCount`) 1))
  (`|ExecutionSequence`
    (:`then_0`
      (`self.Clear`))
    (:`then_1`
      (`self.Initialize`))
    (:`then_5`
      (bind _instancecount (`self.CalcInstanceCount` (`self.DistanceToEnd`) (`self.MeshLength`)))
      (set `self.InstanceCount` _instancecount))
    (:`then_6`
      (for _index (range (+ _returnvalue 1))
        (bind (_index_2 _transform) (`self.AddModule` _index (`self.MeshLength`)))
        (`self.AddDecorations` _transform (`self.MeshLength`) _index_2))
      (for _index_3 (range (+ (`KismetMathLibrary.Clamp` (`self.ConnectorIndexStart`) 0 1) 1))
        (`self.AddModule` (+ _index_3 _returnvalue) (`self.MeshLength`) true)))))

(fn `UserConstructionScript`
  (if (`self.UseInteractiveRefresh`)
    (`self.RunWallGeneration`)))