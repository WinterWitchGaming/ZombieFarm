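; Hedge maze room door that opens once its blood score, shown on a widget and material bar, reaches a threshold.
; Opening ends the room in GM_HedgeMaze, spawns enemy spawners for the next room, removes the old room's and destroys all blood vials.
; A timeline slides the door down.
; When the player overlaps the open door's trigger, it closes, turns on blocking collision and signals the game mode to start the next room.
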(event `self.ReceiveBeginPlay`
  (bind _asgm_hedge_maze (cast `/Game/FrameWork/GameModes/GM_HedgeMaze` (`GameplayStatics.GetGameMode`)))
  (set `self.Game Mode REF` _asgm_hedge_maze)
  (bind _asui_door (cast `/Game/Maps/MapFunctionality/UI_Door` (`WidgetComponent.GetWidget` (`self.Blood Bar`))))
  (set `self.UI REF` _asui_door))

(event `/Game/Maps/MapFunctionality/BPI_MapFunctionality.Add to score of door`
  (params (`Score to add` :type "Float (double-precision)"))
  (bind _returnvalue (/ (`self.Score`) (`self.Score needed to open`)))
  (bind _output_get (set `self.Score` (+ (`self.Score`) `Score to add`)))
  (`/Game/Maps/MapFunctionality/UI_Door.UpdateBloodBar` (`self.UI REF`) _returnvalue)
  (`MaterialInstanceDynamic.SetScalarParameterValue` (`self.BloodBarMatInstance`) "Level" (- 1.0 _returnvalue))
  (if (>= _output_get (`self.Score needed to open`))
    (`self.Open Door`)))

(event `Open Door`
  (bind _cube (`self.Cube`))
  (bind (_relativelocation_x _relativelocation_y _relativelocation_z) (`KismetMathLibrary.BreakVector` (`SceneComponent.RelativeLocation` _cube)))
  (`|ExecutionSequence`
    (:`then_0`
      (`/Game/FrameWork/GameModes/GM_HedgeMaze.End Room` (`self.Game Mode REF`) (`self.Room to open`))
      (`self.Create New Spawners`)
      (`self.Destroy old Spawners`)
      (set `self.Door open?` true)
      (set `self.Start LOC` (`SceneComponent.RelativeLocation` _cube))
      (`GameplayStatics.PlaySoundAtLocation` "/Game/Maps/MapFunctionality/doorSlideRandomizer.doorSlideRandomizer" (0.0 0.0 0.0) (struct) 1.0 1.0 0.0 null null null null)
      (bind (_direction _newtrack_0) (`Timeline|Move Door TL` :!via `PlayFromStart` :!label _label)
        (:`Update`
          (`SceneComponent.K2_SetRelativeLocation` _cube (`KismetMathLibrary.VLerp` (`self.Start LOC`) (`KismetMathLibrary.MakeVector` _relativelocation_x _relativelocation_y (- _relativelocation_z 150.0)) _newtrack_0) false false))))
    (:`then_1`
      (bind _outactors (`GameplayStatics.GetAllActorsOfClass` "/Game/Maps/MapFunctionality/BloodVial/BP_BloodVial.BP_BloodVial_C"))
      (for _array_element _outactors
        (`/Game/Maps/MapFunctionality/BloodVial/BP_BloodVial.Destroy vial` _array_element)))))

(event `Close Door`
  (goto _label :!via `ReverseFromEnd`))

(event `self.Box.OnComponentBeginOverlap`
  (params (OverlappedComponent :type "PrimitiveComponent Object Reference") (OtherActor :type "Actor Object Reference") (OtherComp :type "PrimitiveComponent Object Reference") (OtherBodyIndex :type Integer) (bFromSweep :type Boolean) (SweepResult :type "HitResult Structure (by ref)"))
  (if (`self.Door open?`)
    (`/Engine/EditorBlueprintResources/StandardMacros.IsValid` OtherActor
      (:`Is Valid`
        (if (`self.ActorHasTag` OtherActor "Player")
          (`self.Close Door`)
          (`GameplayStatics.PlaySoundAtLocation` "/Game/Maps/MapFunctionality/doorSlideRandomizer.doorSlideRandomizer" (0.0 0.0 0.0) (struct) 1.0 1.0 0.0 null null null null)
          (message `/Game/FrameWork/GameModes/BPI_OnGameMode.Start Next room` (`GameplayStatics.GetGameMode`) (`self.Room to open`))
          (set `self.Door open?` false)
          (`PrimitiveComponent.SetCollisionResponseToAllChannels` (`self.Box1`) "ECR_Block"))))))

(fn `Create New Spawners`
  (bind _outactors (`GameplayStatics.GetAllActorsOfClass` "/Game/Maps/MapFunctionality/BP_NewEnemySpawnerLOC.BP_NewEnemySpawnerLOC_C"))
  (for _array_element _outactors
    (if (== (`/Game/Maps/MapFunctionality/BP_NewEnemySpawnerLOC.RoomNumber` _array_element) (`self.Room to open`))
      (`|SpawnActorFromClass` "/Game/Enemies/Spawner/BP_EnemySpawner.BP_EnemySpawner_C" (`self.GetTransform` _array_element) "Undefined" "MultiplyWithRoot" null (`self.Room to open`) null))))

(fn `Destroy old Spawners`
  (bind _outactors (`GameplayStatics.GetAllActorsOfClass` "/Game/Enemies/Spawner/BP_EnemySpawner.BP_EnemySpawner_C"))
  (for _array_element _outactors
    (if (== (`/Game/Enemies/Spawner/BP_EnemySpawner.Room Number` _array_element) (`self.Room to close`))
      (`self.K2_DestroyActor` _array_element))))

(fn `UserConstructionScript`
  (bind _returnvalue (`KismetMaterialLibrary.CreateDynamicMaterialInstance` "/Game/Materials/M_BloodBar.M_BloodBar" "None"))
  (`PrimitiveComponent.SetMaterial` (`self.Cube`) 2 _returnvalue)
  (set `self.BloodBarMatInstance` _returnvalue))