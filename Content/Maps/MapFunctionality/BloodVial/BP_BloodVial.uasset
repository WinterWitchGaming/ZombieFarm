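; BP_BloodVial is a blood vial pickup that adds to a door score when touched.
; On sphere overlap with any valid actor, it reads a blood multiplier from the game mode and sends that actor a score message with a base amount plus a multiplier-scaled bonus.
; It then spawns a Niagara effect at its location and destroys itself.
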(event `self.Sphere.OnComponentBeginOverlap`
  (params (OverlappedComponent :type "PrimitiveComponent Object Reference") (OtherActor :type "Actor Object Reference") (OtherComp :type "PrimitiveComponent Object Reference") (OtherBodyIndex :type Integer) (bFromSweep :type Boolean) (SweepResult :type "HitResult Structure (by ref)"))
  (`/Engine/EditorBlueprintResources/StandardMacros.IsValid` OtherActor
    (:`Is Valid`
      (bind _blood_multiplier (message `/Game/FrameWork/GameModes/BPI_OnGameMode.GetBloodMultiplier` (`GameplayStatics.GetGameMode`)))
      (message `/Game/Maps/MapFunctionality/BPI_MapFunctionality.Add to score of door` OtherActor (+ 10.0 (* _blood_multiplier 10.0)))
      (`self.Destroy vial`))))

(event `Destroy vial`
  (`NiagaraFunctionLibrary.SpawnSystemAtLocation` "/Game/Maps/MapFunctionality/BloodVial/NS_BloodVial.NS_BloodVial" (`self.K2_GetActorLocation`))
  (`self.K2_DestroyActor`))

(fn `UserConstructionScript`)