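; AC_InteractionSystem is an interaction component that lets the player trigger interactable actors in front of the camera.
; Its Interact event sphere-traces from the player 0 camera along its forward vector over a supplied Range, with timed debug drawing enabled.
; A valid hit actor tagged "Interactable" receives the InteractMessage interface call, which BP_InteractableBase implements, keeping the component decoupled from specific interactable types.
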(event `Interact`
  (params (Range :type "Float (single-precision)"))
  (bind _returnvalue (`GameplayStatics.GetPlayerCameraManager` 0))
  (bind _returnvalue_2 (`PlayerCameraManager.GetCameraLocation` _returnvalue))
  (bind _outhit (`KismetSystemLibrary.SphereTraceSingle` :`Start` _returnvalue_2 :`End` (+ _returnvalue_2 (* (`Actor.GetActorForwardVector` _returnvalue) Range)) :`Radius` 20.0 :`TraceChannel` "TraceTypeQuery3" :`DrawDebugType` "ForDuration"))
  (bind (_bblockinghit _binitialoverlap _time _distance _location _impactpoint _normal _impactnormal _physmat _hitactor) (`GameplayStatics.BreakHitResult` _outhit))
  ;[1 1 1] Check to make sure actor is loaded in memory and has the right tag
  (`/Engine/EditorBlueprintResources/StandardMacros.IsValid` _hitactor
    (:`Is Valid`
      (if (`Actor.ActorHasTag` _hitactor "Interactable")
        ;[1 1 1] Interface implemented on BP_InteractableBase
        (message `/Game/Interactionsystem/BluePrintInterfaces/BPI_InteractionSystem.Interact` _hitactor)))))