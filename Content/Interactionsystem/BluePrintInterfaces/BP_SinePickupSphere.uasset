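; BP_SinePickupSphere is a pickup actor that moves along a sine-driven path and disappears when touched.
; From BeginPlay, two vector timelines drive the Box component's relative location, one forward and one reversed, each restarting the other for an endless loop.
; Any actor overlap destroys it and prints a debug string, since the BP_Player cast is left unconnected.
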(event `self.ReceiveBeginPlay`
  (bind (_direction _sinevector) (`Timeline|sineMovement` :!label _label)
    (:`Update`
      (`SceneComponent.K2_SetRelativeLocation` (`self.Box`) _sinevector false false))
    (:`Finished`
      (bind (_direction_2 _sinevector_2) (`Timeline|sineReverse` :!via `ReverseFromEnd`)
        (:`Update`
          (`SceneComponent.K2_SetRelativeLocation` (`self.Box`) _sinevector_2 false false))
        (:`Finished`
          (goto _label :!via `PlayFromStart`))))))

(event `self.ReceiveActorBeginOverlap`
  (params (OtherActor :type "Actor Object Reference"))
  (`self.K2_DestroyActor`)
  (`KismetSystemLibrary.PrintString` "SphereDeath"))

(fn `UserConstructionScript`
  (`parent.UserConstructionScript`))