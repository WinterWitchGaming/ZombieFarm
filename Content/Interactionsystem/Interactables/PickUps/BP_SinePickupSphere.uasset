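; Power-up pickup that bobs along a timeline-driven path and grants a random power-up when interacted with.
; Two timelines, SineMovement forward and SineReverse backward, alternate endlessly to set the Box component's relative location.
; On BeginPlay it caches the level's BP_PowerUpHandler and starts a fixed lifetime timer, after which it destroys itself.
; Interact calls RandomPowerUp on that handler, plays a pickup sound and destroys the actor.
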(event `self.ReceiveBeginPlay`
  (`parent.ReceiveBeginPlay`)
  (`|ExecutionSequence`
    (:`then_0`
      (bind (_direction _sinevector) (`Timeline|sineMovement` :!label _label)
        (:`Update`
          (`SceneComponent.K2_SetRelativeLocation` (`self.Box`) _sinevector false false))
        (:`Finished`
          (bind (_direction_2 _sinevector_2) (`Timeline|sineReverse` :!via `ReverseFromEnd`)
            (:`Update`
              (`SceneComponent.K2_SetRelativeLocation` (`self.Box`) _sinevector_2 false false))
            (:`Finished`
              (goto _label :!via `PlayFromStart`))))))
    (:`then_1`
      (bind _outactors (`GameplayStatics.GetAllActorsOfClass` "/Game/Maps/MapFunctionality/BP_PowerUpHandler.BP_PowerUpHandler_C"))
      (bind _output (`|GetArrayItem` _outactors))
      (`/Engine/EditorBlueprintResources/StandardMacros.IsValid` _output
        (:`Is Valid`
          (set `self.Power Up Handler` _output))))
    (:`then_2`
      (`KismetSystemLibrary.Delay` 50.0)
      (`self.K2_DestroyActor`))))

(event `/Game/Interactionsystem/BluePrintInterfaces/BPI_InteractionSystem.Interact`
  (`/Game/Maps/MapFunctionality/BP_PowerUpHandler.RandomPowerUp` (`self.Power Up Handler`))
  (`GameplayStatics.PlaySound2D` "/Game/Player/Sounds/pickup.pickup" 0.8 1.0 0.0 null null)
  (`self.K2_DestroyActor`))

(fn `UserConstructionScript`
  (`parent.UserConstructionScript`))