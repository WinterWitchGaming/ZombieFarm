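; Base zombie enemy that chases the nearest Player-tagged actor with AI MoveTo and attacks within its AttackRadius.
; Random attack montages deal damage through a notify-timed sphere trace, and non-lethal hits trigger a reaction montage.
; ACHealthDmg decides death, which ragdolls the body, notifies the GameMode, may spawn a power-up, and spawns blood vials facing the current room's door.
; A confusion power-up state blocks attacks and sends it to a random nearby point.
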(event `/Game/Health_Dmg_System/BlueprintInterface/BPI_Health_Dmg_System.Damage Target`
  (params (`Damage Amount` :type "Float (double-precision)"))
  (bind _returnvalue (`AIBlueprintHelperLibrary.GetAIController` self))
  ;[1 1 1] Damage
  (if (not (`self.dead?`))
    (bind _dead_ (`/Game/Health_Dmg_System/ActorComponent/AC_HealthDmg.Damaged Func` (`self.AC_HealthDmg`) `Damage Amount`))
    (bind _output_get (set `self.dead?` _dead_))
    (if _output_get
      (`|ExecutionSequence`
        (:`then_0`
          (`PrimitiveComponent.SetSimulatePhysics` (`self.Mesh`) true)
          (`self.DetachFromControllerPendingDestroy` self)
          (`PrimitiveComponent.SetCollisionResponseToAllChannels` (`self.CapsuleComponent`) "ECR_Ignore")
          (`PrimitiveComponent.SetCollisionResponseToAllChannels` (`self.Crit spot`) "ECR_Ignore")
          (`PrimitiveComponent.SetCollisionResponseToAllChannels` (`self.Body Spot`) "ECR_Ignore")
          (`PrimitiveComponent.SetCollisionResponseToAllChannels` (`self.Attack Radius`) "ECR_Ignore")
          (`self.Tell GM enemy is killed`)
          (`|ExecutionSequence` :!label _label
            (:`then_0`
              (`KismetSystemLibrary.Delay` 20.0)
              (`self.K2_DestroyActor` self))
            (:`then_1`
              (`/Engine/EditorBlueprintResources/StandardMacros.IsValid` _returnvalue
                (:`Is Valid`
                  (`Controller.StopMovement` _returnvalue))))))
        (:`then_1`
          (`self.Spawn power up`))
        (:`then_2`
          (`self.Spawn Blood vial`)))
      (else
        (`self.Hit reaction`)))))

(event `self.ReceiveBeginPlay`
  ;[1 1 1] Chase player, begin play
  (`self.Chase Player`)
  (`self.Set Max Walk speed and health` 50.0 35.0)
  (bind _outactors (`GameplayStatics.GetAllActorsOfClass` "/Game/Maps/MapFunctionality/BP_PowerUpHandler.BP_PowerUpHandler_C"))
  (bind _output (`|GetArrayItem` _outactors))
  (set `self.Power up handler` _output)
  (if (`/Game/Maps/MapFunctionality/BP_PowerUpHandler.Confused zombies?` _output)
    (`self.Start Confusion`)))

(event `Hit reaction`
  ;[1 1 1] Damage
  (if (`self.is mont NOT playing?`)
    (`|PlayMontage` (`self.Mesh`) "/Game/Enemies/Mixamo/Animaitons/Zombie_Reaction_Hit_Montage.Zombie_Reaction_Hit_Montage"
      (:`OnCompleted`
        _)
      (:`OnInterrupted`
        _))
    (`self.Chase Player`)))

(event `Chase Player`
  ;[1 1 1] Chase player, begin play
  (if (not (`self.dead?`))
    ;;[1 0.75 0] Works with multiplayer
    (bind _outactors (`GameplayStatics.GetAllActorsWithTag` "Player"))
    (`|AIMoveTo` self (0.0 0.0 0.0) (`.ReturnValue` (`GameplayStatics.FindNearestActor` (`self.K2_GetActorLocation`) _outactors)) 150.0
      (:`OnSuccess`
        _)
      (:`OnFail`
        _))
    (if (`self.can attack?`)
      (`KismetSystemLibrary.Delay` (`self.Hit Delay`))
      (`self.Start Attacking`)
      (else
        (`self.Chase Player`)))))

(event `/Game/Enemies/BPI_SetEnemyStats.Kill remaining enemies`
  ;[1 1 1] Damage
  (set `self.dead?` true)
  (`PrimitiveComponent.SetSimulatePhysics` (`self.Mesh`) true)
  (`self.DetachFromControllerPendingDestroy` self)
  (`PrimitiveComponent.SetCollisionResponseToAllChannels` (`self.CapsuleComponent`) "ECR_Ignore")
  (`PrimitiveComponent.SetCollisionResponseToAllChannels` (`self.Crit spot`) "ECR_Ignore")
  (`PrimitiveComponent.SetCollisionResponseToAllChannels` (`self.Body Spot`) "ECR_Ignore")
  (`PrimitiveComponent.SetCollisionResponseToAllChannels` (`self.Attack Radius`) "ECR_Ignore")
  (goto _label))

(event `self.Attack Radius.OnComponentBeginOverlap`
  (params (OverlappedComponent :type "PrimitiveComponent Object Reference") (OtherActor :type "Actor Object Reference") (OtherComp :type "PrimitiveComponent Object Reference") (OtherBodyIndex :type Integer) (bFromSweep :type Boolean) (SweepResult :type "HitResult Structure (by ref)"))
  (bind _returnvalue (`AIBlueprintHelperLibrary.GetAIController` self))
  ;[1 1 1] Attack player
  (`/Engine/EditorBlueprintResources/StandardMacros.IsValid` OtherActor
    (:`Is Valid`
      (if (`self.ActorHasTag` OtherActor "Player")
        (set `self.can attack?` true)
        (`self.Start Attacking`)
        (`/Engine/EditorBlueprintResources/StandardMacros.IsValid` _returnvalue
          (:`Is Valid`
            (`AIController.K2_SetFocus` _returnvalue OtherActor)))))))

(event `Start Confusion`
  (bind _charactermovement (`self.CharacterMovement`))
  ;[1 1 1] Zombie PowerUps
  (set `self.Confused?` true)
  (set `self.Current Walk Speed` (`CharacterMovementComponent.MaxWalkSpeed` _charactermovement))
  (set `CharacterMovementComponent.MaxWalkSpeed` 35.0 _charactermovement)
  (bind _randomlocation (`NavigationSystemV1.K2_GetRandomLocationInNavigableRadius` (`self.K2_GetActorLocation`) 500.0 null null))
  (`|AIMoveTo` self _randomlocation null))

(event `self.Attack Radius.OnComponentEndOverlap`
  (params (OverlappedComponent :type "PrimitiveComponent Object Reference") (OtherActor :type "Actor Object Reference") (OtherComp :type "PrimitiveComponent Object Reference") (OtherBodyIndex :type Integer))
  (bind _returnvalue (`AIBlueprintHelperLibrary.GetAIController` self))
  ;[1 1 1] Attack player
  (`/Engine/EditorBlueprintResources/StandardMacros.IsValid` OtherActor
    (:`Is Valid`
      (if (`self.ActorHasTag` OtherActor "Player")
        (set `self.can attack?` false)
        (`/Engine/EditorBlueprintResources/StandardMacros.IsValid` _returnvalue
          (:`Is Valid`
            (`AIController.K2_ClearFocus` _returnvalue)))))))

(event `End Confusion`
  ;[1 1 1] Zombie PowerUps
  (set `self.Confused?` false)
  (set `CharacterMovementComponent.MaxWalkSpeed` (`self.Current Walk Speed`) (`self.CharacterMovement`))
  (`self.Chase Player`))

(event `Start Attacking`
  (bind _returnvalue (`SceneComponent.K2_GetComponentLocation` (`self.Attack LOC`)))
  ;[1 1 1] Attack player
  (if (and (`self.is mont NOT playing?`) (not (`self.Confused?`)))
    (bind _notifyname (`|PlayMontage` (`self.Mesh`) (`KismetArrayLibrary.Array_Random` (`self.Attack mont`)))
      (:`OnCompleted`
        (if (`self.can attack?`) :!label _label_2
          (`KismetSystemLibrary.Delay` (`self.Hit Delay`))
          (`self.Start Attacking`)
          (else
            (`self.Chase Player`))))
      (:`OnInterrupted`
        (goto _label_2))
      (:`OnNotifyBegin`
        (switch `name` _notifyname
          (:`Attack`
            (bind (_outhit _returnvalue_2) (`KismetSystemLibrary.SphereTraceSingle` _returnvalue _returnvalue 60.0 "TraceTypeQuery2"))
            (if _returnvalue_2
              (bind (_bblockinghit _binitialoverlap _time _distance _location _impactpoint _normal _impactnormal _physmat _hitactor) (`GameplayStatics.BreakHitResult` _outhit))
              (`/Engine/EditorBlueprintResources/StandardMacros.IsValid` _hitactor
                (:`Is Valid`
                  (if (`self.ActorHasTag` _hitactor "Player")
                    (message `/Game/Health_Dmg_System/BlueprintInterface/BPI_Health_Dmg_System.Damage Target` _hitactor 50.0)))))))))
    (else
      (goto _label_2))))

(event `/Game/Enemies/BPI_SetEnemyStats.Set Health Walk Speed`
  (params (Health :type "Float (double-precision)") (`Walk Speed` :type "Float (double-precision)"))
  (`self.Set Max Walk speed and health` Health `Walk Speed`))

(fn `Set Max Walk speed and health`
  (params (Health :type "Float (double-precision)") (`Max Walk Speed` :type "Float (single-precision)"))
  (bind _ac_healthdmg (`self.AC_HealthDmg`))
  (set `/Game/Health_Dmg_System/ActorComponent/AC_HealthDmg.Health` Health _ac_healthdmg)
  (set `/Game/Health_Dmg_System/ActorComponent/AC_HealthDmg.Max Health` Health _ac_healthdmg)
  (set `CharacterMovementComponent.MaxWalkSpeed` (`KismetMathLibrary.FClamp` (`KismetMathLibrary.RandomFloatInRange` (+ `Max Walk Speed` 100.0) (- `Max Walk Speed` 100.0)) 35.0 600.0) (`self.CharacterMovement`)))

(fn `Spawn Blood vial`
  (bind _room_number (message `/Game/FrameWork/GameModes/BPI_OnGameMode.get room number` (`GameplayStatics.GetGameMode`)))
  (bind _outactors (`GameplayStatics.GetAllActorsOfClass` "/Game/Maps/MapFunctionality/BP_Door.BP_Door_C"))
  (for _array_element _outactors
    (if (== (`/Game/Maps/MapFunctionality/BP_Door.Door Number` _array_element) _room_number)
      (`|SpawnActorFromClass` "/Game/Maps/MapFunctionality/BloodVial/BP_BloodVial.BP_BloodVial_C" (`KismetMathLibrary.MakeTransform` (`self.K2_GetActorLocation`) (`KismetMathLibrary.FindLookAtRotation` (`self.K2_GetActorLocation`) (`self.K2_GetActorLocation` _array_element))) "Undefined" "MultiplyWithRoot" null null))))

(fn `Spawn power up`
  (bind _outactors (`GameplayStatics.GetAllActorsOfClass` "/Game/Interactionsystem/Interactables/PickUps/BP_SinePickupSphere.BP_SinePickupSphere_C"))
  (if (and (`KismetMathLibrary.RandomBoolWithWeight` 0.2) (not (`/Game/Maps/MapFunctionality/BP_PowerUpHandler.Pwer up active?` (`self.Power up handler`))) (<= (`KismetArrayLibrary.Array_Length` _outactors) 3))
    (`|SpawnActorFromClass` "/Game/Interactionsystem/Interactables/PickUps/BP_SinePickupSphere.BP_SinePickupSphere_C" (`self.GetTransform`) "Undefined" "MultiplyWithRoot" null null)))

(fn `Tell GM enemy is killed`
  (message `/Game/FrameWork/GameModes/BPI_OnGameMode.Enemy Killed` (`GameplayStatics.GetGameMode`)))

(fn `UserConstructionScript`)