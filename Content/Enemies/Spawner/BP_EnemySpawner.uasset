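; Enemy spawner actor that creates BP_Enemy_Base instances on request through its Spawnenemy event.
; Each enemy appears at a small random horizontal offset from the spawner, high above it, with a random yaw.
; If the spawn succeeds, the given Health and WalkSpeed are passed to the new enemy through a SetHealthWalkSpeed message.
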(event `Spawn enemy`
  (params (Health :type "Float (double-precision)") (`Walk Speed` :type "Float (double-precision)"))
  (bind (_returnvalue_x _returnvalue_y _returnvalue_z) (`KismetMathLibrary.BreakVector` (`self.K2_GetActorLocation`)))
  (bind (_returnvalue_roll _returnvalue_pitch _returnvalue_yaw) (`KismetMathLibrary.BreakRotator` (`KismetMathLibrary.RandomRotator` false)))
  (bind _returnvalue (`|SpawnActorFromClass` "/Game/Enemies/BP_Enemy_Base.BP_Enemy_Base_C" (`KismetMathLibrary.MakeTransform` (`KismetMathLibrary.MakeVector` (`KismetMathLibrary.RandomFloatInRange` (- _returnvalue_x 20.0) (+ _returnvalue_x 20.0)) (`KismetMathLibrary.RandomFloatInRange` (- _returnvalue_y 20.0) (+ _returnvalue_y 20.0)) (+ _returnvalue_z 5000.0)) (`KismetMathLibrary.MakeRotator` 0.0 0.0 _returnvalue_yaw)) "Undefined" "MultiplyWithRoot" null null))
  (`/Engine/EditorBlueprintResources/StandardMacros.IsValid` _returnvalue
    (:`Is Valid`
      (message `/Game/Enemies/BPI_SetEnemyStats.Set Health Walk Speed` _returnvalue Health `Walk Speed`))))

(fn `UserConstructionScript`)