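; BP_BossPillar is a boss-fight pillar that accumulates score in a blood bar to stun BP_Boss.
; AddtoScoreOfDoor updates its UI_Door widget and, at the threshold, stuns the boss and starts the Confused Zombies power-up through BP_PowerUpHandler.
; Score gains are ignored while stunned.
; StartDrainBlood runs a looping timer that lowers the score, ending the stun once it empties.
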(event `self.ReceiveBeginPlay`
  (bind _asui_door (cast `/Game/Maps/MapFunctionality/UI_Door` (`WidgetComponent.GetWidget` (`self.Widget`))))
  (set `self.UI REF` _asui_door)
  (bind _outactors (`GameplayStatics.GetAllActorsOfClass` "/Game/Enemies/BOSS/BP_Boss.BP_Boss_C"))
  (set `self.Boss REF` (`|GetArrayItem` _outactors)))

(event `/Game/Maps/MapFunctionality/BPI_MapFunctionality.Add to score of door`
  (params (`Score to add` :type "Float (double-precision)"))
  (bind _score_needed_to_stun_boss (`self.Score needed to stun boss`))
  (bind _stunned_ (`/Game/Enemies/BOSS/BP_Boss.Stunned?` (`self.Boss REF`)))
  (if (not (`self.Stunned?`))
    (bind _output_get (set `self.Score` (+ (`self.Score`) `Score to add`)))
    (`/Game/Maps/MapFunctionality/UI_Door.UpdateBloodBar` (`self.UI REF`) (/ _output_get _score_needed_to_stun_boss))
    (if (and (>= _output_get _score_needed_to_stun_boss) (not _stunned_))
      (`/Game/Enemies/BOSS/BP_Boss.Stun boss` (`self.Boss REF`))
      (set `self.Stunned?` _stunned_)
      (bind _outactors (`GameplayStatics.GetAllActorsOfClass` "/Game/Maps/MapFunctionality/BP_PowerUpHandler.BP_PowerUpHandler_C"))
      (`/Game/Maps/MapFunctionality/BP_PowerUpHandler.StartConfusedZombies` (`|GetArrayItem` _outactors) "Confused Zombies" 25))))

(event `Start Drain Blood`
  (bind _returnvalue (`KismetSystemLibrary.K2_SetTimerDelegate` (delegate `Drain Blood`) 0.4 true -0.4))
  (set `self.Blood drain timer` _returnvalue))

(event `Drain Blood`
  (bind _output_get (set `self.Score` (- (`self.Score`) 10.0)))
  (`/Game/Maps/MapFunctionality/UI_Door.UpdateBloodBar` (`self.UI REF`) (/ _output_get (`self.Score needed to stun boss`)))
  (if (<= _output_get 0.0)
    (`KismetSystemLibrary.K2_ClearAndInvalidateTimerHandle` (`self.Blood drain timer`))
    (`/Game/Enemies/BOSS/BP_Boss.Stop being stunned` (`self.Boss REF`))
    (set `self.Stunned?` false)))

(fn `UserConstructionScript`)