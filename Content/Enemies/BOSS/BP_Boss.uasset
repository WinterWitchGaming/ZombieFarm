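; Flying boss that roams between BP_BossPath actors and periodically shoots projectiles at the player.
; A one-second looping timer drives random AI moves and counts down a random value, then the boss flies to the path point nearest the player, focuses and attacks.
; Attacks and damage are gated by the game mode's boss fight flag.
; Damage goes through ACHealthDmg, spawns blood, broadcasts health ratio, and on death triggers the end-game message.
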(event `Fly to attack point`
  (bind _returnvalue (`GameplayStatics.GetPlayerCharacter` 0))
  ;[1 1 1] Attack player
  (`KismetSystemLibrary.K2_ClearAndInvalidateTimerHandle` (`self.Flying Around Timer`))
  (`|AIMoveTo` self (0.0 0.0 0.0) (`.ReturnValue` (`GameplayStatics.FindNearestActor` (`self.K2_GetActorLocation` _returnvalue) (`self.Boss Path Array`))) 10.0
    (:`OnSuccess`
      (`AIController.K2_SetFocus` (`AIBlueprintHelperLibrary.GetAIController` self) _returnvalue)
      (`KismetSystemLibrary.Delay` 1.0)
      (`self.Attack Player`))
    (:`OnFail`
      (`self.Flying Around`))))

(event `self.ReceiveBeginPlay`
  (`CharacterMovementComponent.SetMovementMode` (`self.CharacterMovement`) "MOVE_Flying" 0)
  (bind _outactors (`GameplayStatics.GetAllActorsOfClass` "/Game/Enemies/BOSS/BP_BossPath.BP_BossPath_C"))
  (set `self.Boss Path Array` _outactors)
  (`self.Flying Around`))

(event `Attack Player`
  (bind _returnvalue (`SceneComponent.K2_GetComponentLocation` (`self.Arrow1`)))
  ;[1 1 1] Attack player
  (bind _bossfight_ (message `/Game/FrameWork/GameModes/BPI_OnGameMode.getBossFight?` (`GameplayStatics.GetGameMode`)))
  (if _bossfight_
    (`|SpawnActorFromClass` "/Game/Enemies/BOSS/BP_BossProjectile.BP_BossProjectile_C" (`KismetMathLibrary.MakeTransform` _returnvalue (`KismetMathLibrary.FindLookAtRotation` _returnvalue (`self.K2_GetActorLocation` (`GameplayStatics.GetPlayerCharacter` 0)))) "Undefined" "MultiplyWithRoot" null null)
    (`KismetSystemLibrary.Delay` 1.0)
    (`self.Flying Around`)
    (else
      (`self.Flying Around`))))

(event `Flying Around`
  ;[1 1 1] Fly around
  (set `self.TimeBeforeAttack` (`KismetMathLibrary.RandomIntegerInRange` 5 10))
  (`self.Fly to point`)
  (bind _returnvalue (`KismetSystemLibrary.K2_SetTimerDelegate` (delegate `Fly to point`) 1.0 true -1.0))
  (set `self.Flying Around Timer` _returnvalue))

(event `Fly to point`
  ;[1 1 1] Fly around
  (`AIController.K2_ClearFocus` (`AIBlueprintHelperLibrary.GetAIController` self))
  (bind _result (`/Engine/EditorBlueprintResources/StandardMacros.DecrementInt` (`self.TimeBeforeAttack`))
    (:`  `
      (if (> _result 0)
        (`|AIMoveTo` self (0.0 0.0 0.0) (`KismetArrayLibrary.Array_Random` (`self.Boss Path Array`)) 2.0
          (:`OnSuccess`
            (`AIController.K2_SetFocus` (`AIBlueprintHelperLibrary.GetAIController` self) (`GameplayStatics.GetPlayerCharacter` 0)))
          (:`OnFail`
            (`self.Fly to attack point`)))
        (else
          (`self.Fly to attack point`))))))

(event `/Game/Health_Dmg_System/BlueprintInterface/BPI_Health_Dmg_System.Damage Target`
  (params (`Damage Amount` :type "Float (double-precision)") (`Hit Location` :type "Vector Structure") (`Crit?` :type Boolean))
  (bind _ac_healthdmg (`self.AC_HealthDmg`))
  ;[1 1 1] Damage
  (bind _bossfight_ (message `/Game/FrameWork/GameModes/BPI_OnGameMode.getBossFight?` (`GameplayStatics.GetGameMode`)))
  (if _bossfight_
    (bind _dead_ (`/Game/Health_Dmg_System/ActorComponent/AC_HealthDmg.Damaged Func` (`self.AC_HealthDmg`) `Damage Amount`))
    (`NiagaraFunctionLibrary.SpawnSystemAtLocation` "/Game/Enemies/NS_Blood.NS_Blood" `Hit Location`)
    (if _dead_
      (message `/Game/FrameWork/GameModes/BPI_OnGameMode.End Game` (`GameplayStatics.GetGameMode`))
      (`self.K2_DestroyActor`)
      (else
        (`self.OnHealthChange` (/ (`/Game/Health_Dmg_System/ActorComponent/AC_HealthDmg.Health` _ac_healthdmg) (`/Game/Health_Dmg_System/ActorComponent/AC_HealthDmg.Max Health` _ac_healthdmg)))))))

(fn `UserConstructionScript`)